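; Cat enemy that chases player 0 and attacks at close range, with the behaviour loop written directly in the EventGraph.
; From BeginPlay it repeatedly waits, meows and runs AI MoveTo toward the player, calling TryFistAttack on arrival if within range, then restarting whether the move succeeds or fails.
; BeginPlay also sets the capsule to ignore the Camera collision channel.
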(event EventBeginPlay
  (bind _returnvalue (Game|GetPlayerCharacter 0))
  (Utilities|FlowControl|Sequence
    (:then_0
      (Utilities|FlowControl|Delay 3.0 :!label _label)
      (Audio|PlaySoundatLocation "/Game/Main/InGame/Audios/SFX/A_Cat_Meow_02.A_Cat_Meow_02" (Transformation|GetActorLocation) "0, 0, 0" 1.0 1.0 0.0 0 0 0 0)
      (AI|AIMoveTo self "0, 0, 0" _returnvalue 5.0 false
        (:OnSuccess
          (if (<= (Math|Vector|Distance(Vector) (Transformation|GetActorLocation _returnvalue) (Transformation|GetActorLocation)) 1.5e+02)
            (Class|NxEnemyCat|TryFistAttack)
            (goto _label)
            (else
              (goto _label))))
        (:OnFail
          (goto _label))))
    (:then_1
      (Collision|SetCollisionResponsetoChannel (Variables|Default|GetCapsuleComponent) "ECC_Camera" "ECR_Ignore"))))

(event Collision|EventActorBeginOverlap
  (params (OtherActor :type Actor%20Object%20Reference)))

(event EventTick
  (params (DeltaSeconds :type Float%20%28single-precision%29)))

(fn ConstructionScript)